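; Stage 2 normal portal Blueprint with minimap icon support, though the portal behavior itself is not implemented in this graph.
; NewFunction moves CaleHelper to the actor's location, then sends its relative location as a 2D position to the player HUD's icon-position update message.
; Nothing here calls that function: BeginPlay only checks the minimap icon component's validity, and overlap, Tick and construction are empty.
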(event `self.ReceiveBeginPlay`
  (`self.BaseMiniMap_Icon_com`
    (:`then`)
    (:`else`)))

(event `self.ReceiveTick`
  (params (DeltaSeconds :type "Float (single-precision)")))

(fn `NewFunction`
  (`SceneComponent.K2_SetWorldLocation` (`self.cale_helper`) (`self.K2_GetActorLocation`) false false)
  (message `/Game/Blueprint/UI/Map/MiniMap_IconBp.UodatelconPosition` (`PlayerController.GetHUD` (`GameplayStatics.GetPlayerController` 0)) (`KismetMathLibrary.Conv_VectorToVector2D` (`SceneComponent.RelativeLocation` (`self.cale_helper`)))))

(fn `UserConstructionScript`)