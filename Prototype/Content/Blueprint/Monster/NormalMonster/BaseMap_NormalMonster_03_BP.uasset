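; Normal monster Blueprint for a skeleton knight with a minimap icon and a dissolve death effect.
; On death it hides the minimap icon component and swaps body, armor and weapon to dynamic materials.
; A timeline drives their dissolve amount in step with an edge Niagara effect sharing the same texture.
; Tick still updates the icon position through CalcHelper, but the widget creation and attachment logic is disconnected.
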(event `self.ReceiveBeginPlay`)

(event `self.ReceiveTick`
  (params (DeltaSeconds :type "Float (single-precision)"))
  (`self.Update icon Position`))

(event `MonsterIsDead`
  (bind _p_dissolveedge_pupple (`self.P_DissolveEdge_Pupple`))
  (bind _texture (`self.Texture`))
  (bind _mesh (`self.Mesh`))
  (`|ExecutionSequence`
    (:`then_0`
      (bind _base_mini_map_icon_com (`self.Base Mini Map Icon Com`)
        (:`then`
          (`Widget.SetVisibility` _base_mini_map_icon_com "Hidden"))
        (:`else`)))
    (:`then_1`
      (`NiagaraComponent.SetVariableFloat` (`self.P_DissolveEdge_Pupple`) "User.Width" 0.1)
      ;[1 1 1] 캐릭터 스켈레탈메쉬가 들고있는 Material 0, 1, 2
      (bind _returnvalue (`PrimitiveComponent.CreateDynamicMaterialInstance` _mesh 1 "/Game/SKnight_modular/Skeleton_Knight_07/materials/MatInst/MI_SKnigh_07_armor_Inst.MI_SKnigh_07_armor_Inst" "None"))
      (bind _returnvalue_2 (`PrimitiveComponent.CreateDynamicMaterialInstance` _mesh 0 "/Game/SKnight_modular/Skeleton/materials/MI_Skeleton_Inst.MI_Skeleton_Inst" "None"))
      ;[1 1 1] 스켈레탈메쉬 검, 방패
      (bind _returnvalue_3 (`PrimitiveComponent.CreateDynamicMaterialInstance` (`self.SK_weapon_01`) 0 "/Game/SKnight_modular/Skeleton_Knight_01/materials/MatInst/MI_weapon_01_Inst.MI_weapon_01_Inst" "None"))
      (`MaterialInstanceDynamic.SetTextureParameterValue` _returnvalue "Texture" _texture)
      (`MaterialInstanceDynamic.SetTextureParameterValue` _returnvalue_2 "Texture" _texture)
      (`MaterialInstanceDynamic.SetTextureParameterValue` null "Texture" _texture)
      (`MaterialInstanceDynamic.SetTextureParameterValue` _returnvalue_3 "Texture" _texture)
      (`NiagaraFunctionLibrary.SetTextureObject` (`self.P_DissolveEdge_Pupple`) "Texture" _texture)
      (bind (_direction _time) (`Timeline|타임라인` :!via `PlayFromStart`)
        (:`Update`
          (`MaterialInstanceDynamic.SetScalarParameterValue` _returnvalue "Amount" (`KismetMathLibrary.Lerp` 1.0 0.0 _time))
          (`MaterialInstanceDynamic.SetScalarParameterValue` _returnvalue_3 "Amount" (`KismetMathLibrary.Lerp` 1.0 0.0 _time))
          (`MaterialInstanceDynamic.SetScalarParameterValue` null "Amount" (`KismetMathLibrary.Lerp` 1.0 0.0 _time))
          (`MaterialInstanceDynamic.SetScalarParameterValue` _returnvalue_2 "Amount" (`KismetMathLibrary.Lerp` 1.0 0.0 _time))
          (`NiagaraComponent.SetVariableFloat` _p_dissolveedge_pupple "User.Amount" (`KismetMathLibrary.Lerp` 1.0 0.0 _time)))
        (:`Finished`
          (`NiagaraComponent.SetVariableFloat` _p_dissolveedge_pupple "User.Width" 0.0))))))

(fn `Update icon Position`
  (`SceneComponent.K2_SetWorldLocation` (`self.calc_helper`) (`self.K2_GetActorLocation`) false false)
  (bind _minimap_icon (`self.miniMap_icon`)
    (:`then`
      (`/Game/Blueprint/UI/Map/wdg_stage_01minimap_icon.UpdstelconLocation` _minimap_icon (`KismetMathLibrary.Conv_VectorToVector2D` (`SceneComponent.RelativeLocation` (`self.calc_helper`)))))
    (:`else`)))

(fn `UserConstructionScript`)