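; Boss-monster obstacle actor that shows its own icon on the minimap.
; Shortly after BeginPlay it creates and configures the icon widget, hides it on the destroyed event, and attaches a CalcHelper component to the player's root.
; Every tick it moves CalcHelper to the obstacle's location and feeds its relative location to the icon as a 2D position, using attachment to get player-relative coordinates.
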(event `OnDestroyedEvent_Event`
  ;[1 1 1] 델리게이트 이벤트 구독
  (`Widget.SetVisibility` (stale `self.ReceiveBeginPlay` _output_get) "Hidden"))

(event `self.ReceiveBeginPlay`
  (`KismetSystemLibrary.Delay` 0.2)
  (bind _returnvalue (`|CreateWidget` "/Game/Blueprint/UI/Map/wdg_minimap_icon.wdg_minimap_icon_C"))
  (bind _output_get (set `self.miniMap_icon` _returnvalue))
  (`/Game/Blueprint/UI/Map/wdg_minimap_icon.change Icon` _output_get (`self.icon`))
  (`/Game/Blueprint/UI/Map/wdg_minimap_icon.change size` _output_get (`self.In Size`))
  ;[1 1 1] 델리게이트 이벤트 구독
  (add `self.OnDestroyedEvent` (delegate `OnDestroyedEvent_Event`))
  (`Widget.SetVisibility` _output_get "Visible")
  (`UserWidget.AddToViewport` _output_get 0)
  (`SceneComponent.K2_AttachToComponent` (`self.calc_helper`) (`Actor.RootComponent` (`GameplayStatics.GetPlayerCharacter` 0)) "None" "KeepWorld" "KeepWorld" "KeepWorld" true)
  (`self.Update icon Position`))

(event `self.ReceiveTick`
  (params (DeltaSeconds :type "Float (single-precision)"))
  (`self.Update icon Position`))

(fn `Update icon Position`
  (`SceneComponent.K2_SetWorldLocation` (`self.calc_helper`) (`self.K2_GetActorLocation`) false false)
  (bind _minimap_icon (`self.miniMap_icon`)
    (:`then`
      (`/Game/Blueprint/UI/Map/wdg_minimap_icon.UpdstelconLocation` _minimap_icon (`KismetMathLibrary.Conv_VectorToVector2D` (`SceneComponent.RelativeLocation` (`self.calc_helper`)))))
    (:`else`)))

(fn `UserConstructionScript`)